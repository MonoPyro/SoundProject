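; BP_Drawer is an interactable drawer that slides open and closed, reusing an inherited setup with a Door component.
; BeginPlay stores the Door's world X as the closed position and a fixed offset from it as the open position.
; Interact plays or reverses a timeline that lerps between them, ignoring input until it finishes and toggles the Open state.
; Movement is along world X, independent of the actor's rotation.
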(event `self.ReceiveBeginPlay`
  (bind _returnvalue_x (`KismetMathLibrary.BreakVector` (`SceneComponent.K2_GetComponentLocation` (`self.Door`))))
  (`parent.ReceiveBeginPlay`)
  (set `self.StartPos` _returnvalue_x)
  (set `self.EndPos` (+ _returnvalue_x 50.0)))

(event `/Game/FPMovement/Player/Blueprints/Interface/BP_Interact.Interact`
  (params (Player :type "/Game/FPMovement/Player/Blueprints/BP_Player Object Reference"))
  (bind _door (`self.Door`))
  (bind (_returnvalue_x _returnvalue_y _returnvalue_z) (`KismetMathLibrary.BreakVector` (`SceneComponent.K2_GetComponentLocation` _door)))
  (if (not (`self.bIsOpening`))
    (set `self.bIsOpening` true)
    (if (`self.bOpen?`)
      (bind (_direction _open) (`Timeline|Timeline_1` :!via `ReverseFromEnd` :!label _label)
        (:`Update`
          (`SceneComponent.K2_SetWorldLocation` _door (`KismetMathLibrary.MakeVector` (`KismetMathLibrary.Lerp` (`self.StartPos`) (`self.EndPos`) _open) _returnvalue_y _returnvalue_z) false false))
        (:`Finished`
          (set `self.bOpen?` (not (`self.bOpen?`)))
          (set `self.bIsOpening` false)))
      (else
        (goto _label :!via `PlayFromStart`)))))

(fn `UserConstructionScript`
  (`parent.UserConstructionScript`))