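; BP_CustomText is a Blueprint that displays a configurable Text value through a WBP_CustomText widget hosted in its Widget component.
; The construction script writes Text straight into the widget's CustomText element whenever construction runs.
; On BeginPlay it instead assigns Text to the widget's own Text variable.
; Both paths do nothing if the cast to WBP_CustomText fails.
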(event `self.ReceiveBeginPlay`
  (bind _aswbp_custom_text (cast `/Game/Custom/Widgets/WBP_CustomText` (`WidgetComponent.GetWidget` (`self.Widget`))))
  (set `/Game/Custom/Widgets/WBP_CustomText.Text` (`self.Text`) _aswbp_custom_text))

(fn `UserConstructionScript`
  (bind _aswbp_custom_text (cast `/Game/Custom/Widgets/WBP_CustomText` (`WidgetComponent.GetWidget` (`self.Widget`))))
  (set `TextBlock.Text` (`self.Text`) (`/Game/Custom/Widgets/WBP_CustomText.CustomText` _aswbp_custom_text)))