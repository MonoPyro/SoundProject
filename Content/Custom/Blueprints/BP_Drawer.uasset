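; BP_Drawer is an interactable drawer that slides its static mesh open and closed along the world X axis.
; BeginPlay records the mesh's X position and a fixed offset end point, which a timeline interpolates between.
; Interact plays that timeline forward or in reverse based on a toggled Open flag, ignoring input while it moves.
; The interaction query functions return false and no prompt.
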(event `self.ReceiveBeginPlay`
  (bind _returnvalue_x (`KismetMathLibrary.BreakVector` (`SceneComponent.K2_GetComponentLocation` (`self.StaticMesh`))))
  (set `self.StartPos` _returnvalue_x)
  (set `self.EndPos` (+ _returnvalue_x 400.0)))

(event `/Game/FPMovement/Player/Blueprints/Interface/BP_Interact.Interact`
  (params (Player :type "/Game/FPMovement/Player/Blueprints/BP_Player Object Reference"))
  (if (not (`self.bIsOpening`))
    (set `self.bIsOpening` true)
    (if (`self.bOpen?`)
      (bind (_direction _open) (`Timeline|Open` :!via `PlayFromStart` :!label _label)
        (:`Update`
          (`SceneComponent.K2_SetWorldLocation` (`self.StaticMesh`) (`KismetMathLibrary.MakeVector` (`KismetMathLibrary.Lerp` (`self.StartPos`) (`self.EndPos`) _open)) false false))
        (:`Finished`
          (set `self.bOpen?` (not (`self.bOpen?`)))
          (set `self.bIsOpening` false)))
      (else
        (goto _label :!via `ReverseFromEnd`)))))

(fn `Can_Interact?`
  (returns (`CanInteract?` :type Boolean))
  (return false))

(fn `Interact_Prompt`
  (returns (`ShowPrompt?` :type Boolean) (Name :type Name))
  (return false "None"))

(fn `UserConstructionScript`)