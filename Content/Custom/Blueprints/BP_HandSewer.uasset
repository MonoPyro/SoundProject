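; BP_HandSewer is an interactable that records a HandSewer flag and opens a warp gallery screen when the player uses it.
; Its Interact override sets that flag on the GI_Custom game instance, runs the parent interaction, then disables the player's input.
; It then creates the WBP_WarpGallery widget and adds it to the viewport, with no logic here to restore input.
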(event `/Game/FPMovement/Player/Blueprints/Interface/BP_Interact.Interact`
  (params (Player :type "/Game/FPMovement/Player/Blueprints/BP_Player Object Reference"))
  (bind _asgi_custom (cast `/Game/Custom/Blueprints/GI_Custom` (`GameplayStatics.GetGameInstance`)))
  (set `/Game/Custom/Blueprints/GI_Custom.HandSewer` true _asgi_custom)
  (`parent.Interact` Player)
  (`self.DisableInput` Player (`GameplayStatics.GetPlayerController` 0))
  (bind _returnvalue (`|CreateWidget` "/Game/Custom/Widgets/WBP_WarpGallery.WBP_WarpGallery_C"))
  (`UserWidget.AddToViewport` _returnvalue 0))

(fn `UserConstructionScript`
  (`parent.UserConstructionScript`))