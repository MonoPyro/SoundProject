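; BP_HandHouse is an interactable that opens a warp gallery UI when the player uses it.
; On Interact it sets the HandHouse flag on GI_Custom, calls the parent interaction, disables player input, then adds a WBP_WarpGallery widget to the viewport.
; If the game instance is not a GI_Custom, the interaction does nothing, including the parent call.
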(event `self.ReceiveBeginPlay`
  (`parent.ReceiveBeginPlay`))

(event `/Game/FPMovement/Player/Blueprints/Interface/BP_Interact.Interact`
  (params (Player :type "/Game/FPMovement/Player/Blueprints/BP_Player Object Reference"))
  (bind _asgi_custom (cast `/Game/Custom/Blueprints/GI_Custom` (`GameplayStatics.GetGameInstance`)))
  (set `/Game/Custom/Blueprints/GI_Custom.HandHouse` true _asgi_custom)
  (`parent.Interact` Player)
  (`self.DisableInput` Player (`GameplayStatics.GetPlayerController` 0))
  (set `/Game/FPMovement/Player/Blueprints/BP_Player.InputEnabled` false Player)
  (bind _returnvalue (`|CreateWidget` "/Game/Custom/Widgets/WBP_WarpGallery.WBP_WarpGallery_C"))
  (`UserWidget.AddToViewport` _returnvalue 0))

(fn `UserConstructionScript`
  (`parent.UserConstructionScript`))