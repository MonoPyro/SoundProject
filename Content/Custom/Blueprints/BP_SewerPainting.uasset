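; BP_SewerPainting is an interactable painting that sends the player into the Medieval_Sewer_Dungeon level.
; On BeginPlay it destroys itself if the game instance's HandSubway flag is set, otherwise it caches the player.
; Interacting shows a HUD notification, turns off further interaction, blends the view to its camera and disables input.
; A timer matching the two-second blend then opens the dungeon level.
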(event `self.ReceiveBeginPlay`
  (bind _asgi_custom (cast `/Game/Custom/Blueprints/GI_Custom` (`GameplayStatics.GetGameInstance`)))
  (if (`/Game/Custom/Blueprints/GI_Custom.HandSubway` _asgi_custom)
    (`self.K2_DestroyActor`)
    (else
      (bind _asbp_player (cast `/Game/FPMovement/Player/Blueprints/BP_Player` (`GameplayStatics.GetPlayerCharacter` 0)))
      (set `self.Player Reference` _asbp_player))))

(event `self.Interact`
  (params (Player :type "/Game/FPMovement/Player/Blueprints/BP_Player Object Reference"))
  (`/Game/FPMovement/Player/Widgets/WB_PlayerHud.AddNotification` (`/Game/FPMovement/Player/Blueprints/BP_Player.WP_PlayerHUD` Player) (`self.Pickup Notification`) (`KismetTextLibrary.Conv_NameToText` (`self.Item Name`)) (`self.Item Color Notification`))
  (set `/Game/FPMovement/Player/Blueprints/BP_Player.ShowPrompt?` false Player)
  (set `self.CanInteract?` false)
  (`self.GoInSubway`))

(event `GoInSubway`
  (`PlayerController.SetViewTargetWithBlend` (`GameplayStatics.GetPlayerController` 0) (`self.Camera`) 2.0 "VTBlend_Linear" 0.0 false)
  (`self.DisableInput` (`self.Player Reference`) (`GameplayStatics.GetPlayerController` 0))
  (`KismetSystemLibrary.K2_SetTimerDelegate` (delegate `ChangeLevel`) 2.0))

(event `ChangeLevel`
  (`GameplayStatics.OpenLevelBySoftObjectPtr` "/Game/Custom/Maps/Medieval_Sewer_Dungeon.Medieval_Sewer_Dungeon"))

(fn `Can_Interact?`
  (returns (`CanInteract?` :type Boolean))
  (return (`self.CanInteract?`)))

(fn `Interact_Prompt`
  (returns (`ShowPrompt?` :type Boolean) (Name :type Name))
  (return (`self.Show Item Prompt?`) (`self.Item Name`)))

(fn `UserConstructionScript`)