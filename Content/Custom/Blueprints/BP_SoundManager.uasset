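; Sound manager actor that plays moving subway audio passes, starting at BeginPlay.
; Each pass randomly picks one of two sides, spawns SC_Subway attached to a Scene component, and sweeps it along X with a timeline, in opposite directions per side.
; An audio-finished callback triggers another pass after a short random delay, but is bound only to the first spawned sound.
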(event `self.ReceiveBeginPlay`
  (`self.Sound`)
  (add `AudioComponent.OnAudioFinished` (`self.SoundPlayed`) (delegate `SoundLoop`)))

(event `SoundLoop`
  (`KismetSystemLibrary.Delay` (`KismetMathLibrary.RandomFloatInRange` 3.0 5.0))
  (`self.Sound`))

(event `Sound`
  (bind _scene (`self.Scene`))
  (bind _location (`self.Location`))
  (bind _location_2 (`self.Location`))
  (switch `int` (`KismetMathLibrary.RandomIntegerInRange` 0 1)
    (:`0`
      (bind _returnvalue (`GameplayStatics.SpawnSoundAttached` "/Game/Custom/Sounds/SC_Subway.SC_Subway" _scene "None" (0.0 0.0 0.0) (struct) "KeepRelativeOffset" false 1.0 1.0 0.0 null null))
      (set `self.SoundPlayed` _returnvalue)
      (bind (_direction _alpha) (`Timeline|Movement`)
        (:`Update`
          (`SceneComponent.K2_SetWorldLocation` (`self.Scene`) (`KismetMathLibrary.MakeVector` (`KismetMathLibrary.Lerp` _location_2 (* _location_2 -1.0) _alpha) 655.0 120.0) false false))))
    (:`1`
      (bind _returnvalue_2 (`GameplayStatics.SpawnSoundAttached` "/Game/Custom/Sounds/SC_Subway.SC_Subway" _scene "None" (0.0 0.0 0.0) (struct) "KeepRelativeOffset" false 1.0 1.0 0.0 null null))
      (set `self.SoundPlayed` _returnvalue_2)
      (bind (_direction_2 _alpha_2) (`Timeline|Movement2`)
        (:`Update`
          (`SceneComponent.K2_SetWorldLocation` (`self.Scene`) (`KismetMathLibrary.MakeVector` (`KismetMathLibrary.Lerp` (* _location -1.0) _location _alpha_2) -655.0 120.0) false false))))))

(fn `UserConstructionScript`)