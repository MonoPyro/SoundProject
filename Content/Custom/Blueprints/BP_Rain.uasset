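; BP_Rain is a spline-based ambient sound actor that plays looping rain from the point on its spline closest to the player.
; BeginPlay caches the BP_Player pawn, sets a configurable tick interval, and assigns the sound and attenuation to the LoopingRain audio component before playing it.
; Each tick reattaches that component to the spline and moves it to the closest point.
; An optional debug mode draws that point, the actor's name and an attenuation sphere.
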(event `self.ReceiveTick`
  (params (DeltaSeconds :type "Float (single-precision)"))
  (`self.Find Closest Point`))

(event `self.ReceiveBeginPlay`
  (`|ExecutionSequence`
    (:`then_0`
      (bind _asbp_player (cast `/Game/FPMovement/Player/Blueprints/BP_Player` (`GameplayStatics.GetPlayerPawn` 0)))
      (set `self.As BP Player` _asbp_player))
    (:`then_1`
      (`self.SetActorTickInterval` (`self.TickInterval`)))
    (:`then_2`
      (`AudioComponent.SetSound` (`self.LoopingRain`) (`self.LoopingSound`))
      (set `AudioComponent.AttenuationSettings` (`self.SoundAttenuation`) (`self.LoopingRain`)))
    (:`then_3`
      (`AudioComponent.Play` (`self.LoopingRain`) 0.0))))

(event `Find Closest Point`
  (bind _soundattenuation (`self.SoundAttenuation`))
  (bind (_attenuation_battenuate _attenuation_bspatialize _attenuation_battenuatewithlpf _attenuation_benablelistenerfocus _attenuation_benablefocusinterpolation _attenuation_benableocclusion _attenuation_busecomplexcollisionforocclusion _attenuation_benablereverbsend _attenuation_benablepriorityattenuation _attenuation_bapplynormalizationtostereosounds _attenuation_benablelogfrequencyscaling _attenuation_benablesubmixsends _attenuation_benablesourcedataoverride _attenuation_benablesendtoaudiolink _attenuation_spatializationalgorithm _attenuation_audiolinksettingsoverride _attenuation_binauralradius _attenuation_customlowpassairabsorptioncurve _attenuation_customhighpassairabsorptioncurve _attenuation_absorptionmethod _attenuation_occlusiontracechannel _attenuation_reverbsendmethod _attenuation_priorityattenuationmethod _attenuation_nonspatializedradiusstart _attenuation_nonspatializedradiusend _attenuation_nonspatializedradiusmode _attenuation_stereospread _attenuation_lpfradiusmin _attenuation_lpfradiusmax _attenuation_lpffrequencyatmin _attenuation_lpffrequencyatmax _attenuation_hpffrequencyatmin _attenuation_hpffrequencyatmax _attenuation_focusazimuth _attenuation_nonfocusazimuth _attenuation_focusdistancescale _attenuation_nonfocusdistancescale _attenuation_focuspriorityscale _attenuation_nonfocuspriorityscale _attenuation_focusvolumeattenuation _attenuation_nonfocusvolumeattenuation _attenuation_focusattackinterpspeed _attenuation_focusreleaseinterpspeed _attenuation_occlusionlowpassfilterfrequency _attenuation_occlusionvolumeattenuation _attenuation_occlusioninterpolationtime _attenuation_reverbwetlevelmin _attenuation_reverbwetlevelmax _attenuation_reverbdistancemin _attenuation_reverbdistancemax _attenuation_manualreverbsendlevel _attenuation_priorityattenuationmin _attenuation_priorityattenuationmax _attenuation_priorityattenuationdistancemin _attenuation_priorityattenuationdistancemax _attenuation_manualpriorityattenuation _attenuation_customreverbsendcurve _attenuation_submixsendsettings _attenuation_custompriorityattenuationcurve _attenuation_pluginsettings _attenuation_distancealgorithm _attenuation_attenuationshape _attenuation_falloffmode _attenuation_dbattenuationatmax _attenuation_attenuationshapeextents _attenuation_coneoffset _attenuation_falloffdistance) (break `SoundAttenuationSettings` (`SoundAttenuation.Attenuation` _soundattenuation)))
  (bind _returnvalue (`SplineComponent.FindLocationClosestToWorldLocation` (`self.Spline`) (`self.K2_GetActorLocation` (`self.As BP Player`)) "World"))
  (`|ExecutionSequence`
    (:`then_0`
      (`SceneComponent.K2_AttachToComponent` (`self.LoopingRain`) (`self.Spline`) "None" "KeepRelative" "KeepRelative" "KeepRelative" true)
      (`SceneComponent.K2_SetWorldLocation` (`self.LoopingRain`) (`SplineComponent.FindLocationClosestToWorldLocation` (`self.Spline`) (`self.K2_GetActorLocation` (`self.As BP Player`)) "World") false false))
    (:`then_1`
      (if (`self.Debug?`)
        (`KismetSystemLibrary.DrawDebugSphere` _returnvalue 100.0 12 (struct :`B` 1.0 :`A` 1.0) 0.2 4.0)
        (`KismetSystemLibrary.DrawDebugString` (+ _returnvalue (0.0 0.0 150.0)) (`KismetSystemLibrary.GetDisplayName` self) null (struct :`B` 1.0 :`A` 1.0) 0.2)
        (`/Engine/EditorBlueprintResources/StandardMacros.IsValid` _soundattenuation
          (:`Is Valid`
            (`KismetSystemLibrary.DrawDebugSphere` _returnvalue _attenuation_falloffdistance 12 (struct :`R` 1.0 :`G` 0.25 :`A` 1.0))))))))

(fn `UserConstructionScript`)