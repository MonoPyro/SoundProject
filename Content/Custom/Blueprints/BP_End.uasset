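; BP_End is a level-end trigger that fades in an end screen as the player approaches it.
; On BeginPlay it caches the BP_Player pawn and adds a WBP_End widget to the viewport.
; Tick drives the widget's background opacity from player distance within an outer radius, increasing with proximity.
; At close range, a DoOnce disables player input, makes the background fully opaque and plays the widget's Anim.
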(event `self.ReceiveBeginPlay`
  (bind _asbp_player (cast `/Game/FPMovement/Player/Blueprints/BP_Player` (`GameplayStatics.GetPlayerPawn` 0)))
  (set `self.PlayerRef` _asbp_player)
  (bind _returnvalue (`|CreateWidget` "/Game/Custom/Widgets/WBP_End.WBP_End_C"))
  (bind _output_get (set `self.HUDEnd` _returnvalue))
  (`UserWidget.AddToViewport` _output_get 0))

(event `self.ReceiveTick`
  (params (DeltaSeconds :type "Float (single-precision)"))
  (bind _playerref (`self.PlayerRef`))
  (bind _returnvalue (`self.GetDistanceTo` (`self.PlayerRef`)))
  (if (<= _returnvalue 1000.0)
    (if (<= _returnvalue 75.0)
      (`/Engine/EditorBlueprintResources/StandardMacros.DoOnce` false
        (:`Completed`
          (`self.DisableInput` _playerref (`GameplayStatics.GetPlayerController` 0))
          (set `/Game/FPMovement/Player/Blueprints/BP_Player.InputEnabled` false _playerref)
          (`Image.SetOpacity` (`/Game/Custom/Widgets/WBP_End.Background` (`self.HUDEnd`)) 1.0)
          (`/Game/Custom/Widgets/WBP_End.Anim` (`self.HUDEnd`))))
      (else
        (`Image.SetOpacity` (`/Game/Custom/Widgets/WBP_End.Background` (`self.HUDEnd`)) (+ (* (/ _returnvalue 1000.0) -1.0) 1.1))))))

(fn `UserConstructionScript`)