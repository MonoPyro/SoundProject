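; BP_HandTrigger is a trigger that snaps a referenced hand actor between two positions when the player enters its box.
; On BeginPlay it stores the hand's location and a second one offset along world X.
; Each player overlap alternates the hand between them through a FlipFlop, with a DoOnce that resets after a short delay to debounce re-triggering.
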(event `self.ReceiveBeginPlay`
  (bind _output_get (set `self.FirstLoc` (`self.K2_GetActorLocation` (`self.HandRef`))))
  (set `self.SecondLoc` (+ _output_get (400.0 0.0 0.0))))

(event `self.Box.OnComponentBeginOverlap`
  (params (OverlappedComponent :type "PrimitiveComponent Object Reference") (OtherActor :type "Actor Object Reference") (OtherComp :type "PrimitiveComponent Object Reference") (OtherBodyIndex :type Integer) (bFromSweep :type Boolean) (SweepResult :type "HitResult Structure (by ref)"))
  (cast `/Game/FPMovement/Player/Blueprints/BP_Player` OtherActor)
  (`/Engine/EditorBlueprintResources/StandardMacros.DoOnce` false :!label _label
    (:`Completed`
      (`/Engine/EditorBlueprintResources/StandardMacros.FlipFlop`
        (:`A`
          (bind _handref (`self.HandRef`)
            (:`then`
              (`self.K2_SetActorLocation` _handref (`self.SecondLoc`) false false))
            (:`else`)))
        (:`B`
          (bind _handref_2 (`self.HandRef`)
            (:`then`
              (`self.K2_SetActorLocation` _handref_2 (`self.FirstLoc`) false false))
            (:`else`))))
      (`KismetSystemLibrary.Delay` 0.5)
      (goto _label :!via `Reset`))))

(fn `UserConstructionScript`)