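; BP_DoorGallery is a gallery door actor that swaps its static mesh to a door frame and plays a glass-breaking sound at its location.
; BeginPlay triggers the break unconditionally.
; A check of the HandSewer, HandSubway and HandHouse flags on the GI_Custom game instance leads into the same break, but no event drives it, so it never runs.
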(event `self.ReceiveBeginPlay`
  (`StaticMeshComponent.SetStaticMesh` (`self.StaticMeshComponent0`) "/Game/Custom/Assets/DoorFrame.DoorFrame")
  (`GameplayStatics.PlaySoundAtLocation` "/Game/Custom/Sounds/glass-breaking.glass-breaking" (`self.K2_GetActorLocation`) (struct) 1.0 1.0 0.0 null null null null))

(fn `UserConstructionScript`)